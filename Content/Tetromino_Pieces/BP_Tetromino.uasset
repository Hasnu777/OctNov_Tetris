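; BP_Tetromino is a Tetris piece actor that drops itself through the level and requests the next piece when it lands.
; After a short delay on BeginPlay, it switches to a falling state and starts a looping timer that steps it downward with a swept move.
; On a blocking hit it changes state, stops the timer and calls SpawnNewPiece on TetrisGameMode, printing debug messages along the way.
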(event Custom|DropTick
  (if (Utilities|Enum|Equal(Enum) (Variables|Default|GetCurrentState) "NewEnumerator1")
    (bind _sweephitresult (Transformation|SetActorLocation (- (Transformation|GetActorLocation) "0.000000,0.000000,100.000000") true false))
    (if (.bBlockingHit (Collision|BreakHitResult _sweephitresult))
      (Variables|Default|SetCurrentState "NewEnumerator2")
      (Utilities|Time|ClearandInvalidateTimerbyHandle (Variables|Default|GetDropTimerHandle))
      (Development|PrintString "1 - FLOOR HIT")
      (bind _astetris_game_mode (Utilities|Casting|CastToTetrisGameMode (Game|GetGameMode))
        (:then
          (Development|PrintString "2 - CAST SUCCESS")
          (Default|SpawnNewPiece _astetris_game_mode))
        (:CastFailed
          (Development|PrintString "CAST FAILED"))))))

(event EventBeginPlay
  (Variables|Default|SetCurrentState "NewEnumerator0")
  (Utilities|FlowControl|Delay 1.5)
  (Variables|Default|SetCurrentState "NewEnumerator1")
  (bind _returnvalue (Utilities|Time|SetTimerbyFunctionName 0 "DropTick" 0.1 true))
  (Variables|Default|SetDropTimerHandle _returnvalue))

(event Collision|EventActorBeginOverlap
  (params (OtherActor :type Actor%20Object%20Reference)))

(event EventTick
  (params (DeltaSeconds :type Float%20%28single-precision%29)))

(fn ConstructionScript)